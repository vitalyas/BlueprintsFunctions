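; PointLight is a Blueprint that blinks its point light a limited number of times when play begins.
; A DoN node capped by BlinksCount drives a loop that waits BlinkDuration, hides the light, waits again, shows it, then re-enters the node.
; A SetVisibility helper function toggles the PointLight component without propagating to children.
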(event `self.ReceiveBeginPlay`
  (`/Engine/EditorBlueprintResources/StandardMacros.Do N` (`self.BlinksCount`) :!label _label
    (:`Exit`
      (`KismetSystemLibrary.Delay` (`self.BlinkDuration`))
      (`self.SetVisibility` false)
      (`KismetSystemLibrary.Delay` (`self.BlinkDuration`))
      (`self.SetVisibility` true)
      (goto _label))))

(fn `SetVisibility`
  (params (isVisible :type Boolean))
  (`SceneComponent.SetVisibility` (`self.PointLight`) isVisible false))

(fn `UserConstructionScript`)